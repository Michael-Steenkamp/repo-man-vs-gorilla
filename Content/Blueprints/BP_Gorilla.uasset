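; BP_Gorilla is a player-controlled gorilla character with a health HUD and a montage-driven attack.
; It creates the health widget at BeginPlay and adds its Enhanced Input mapping on possession for camera-relative movement and look.
; Attack input plays an arm montage, with a DoOnce blocking repeats until it completes or is interrupted.
; The GorillaArm component damages any actor it begins overlapping, independent of the attack state.
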(event OnComponentBeginOverlap(GorillaArm)
  (params (OverlappedComponent :type Primitive%20Component%20Object%20Reference) (OtherActor :type Actor%20Object%20Reference) (OtherComp :type Primitive%20Component%20Object%20Reference) (OtherBodyIndex :type Integer) (bFromSweep :type Boolean) (SweepResult :type Hit%20Result%20Structure%20%28by%20ref%29))
  (Game|Damage|ApplyDamage OtherActor 1.0 0 self))

(event Input|EnhancedActionEvents|EnhancedInputActionIA_Move
  (params (ActionValue :type Vector%202D%20Structure) (ElapsedSeconds :type Float%20%28double-precision%29) (TriggeredSeconds :type Float%20%28double-precision%29) (InputAction :type Input%20Action%20Object%20Reference :default "/Game/Input/IA_Move.IA_Move"))
  (bind _returnvalue (Pawn|GetControlRotation :!class /Script/Engine.Pawn))
  ;[0.15 0.15 0.15 0.5] Add Movement Input to Gorilla
  ;;[0.15 0.15 0.15 0.5] Move left and right
  (Pawn|Input|AddMovementInput (Math|Vector|GetRightVector (Math|Rotator|MakeRotator (.roll _returnvalue) 0.0 (.yaw _returnvalue))) (.x ActionValue) false)
  ;;[0.15 0.15 0.15 0.5] Move forwards and backwards
  (Pawn|Input|AddMovementInput (Math|Vector|GetForwardVector (Math|Rotator|MakeRotator 0.0 0.0 (.yaw (Pawn|GetControlRotation :!class /Script/Engine.Pawn)))) (.y ActionValue) false))

(event Input|EnhancedActionEvents|EnhancedInputActionIA_Look
  (params (ActionValue :type Vector%202D%20Structure) (ElapsedSeconds :type Float%20%28double-precision%29) (TriggeredSeconds :type Float%20%28double-precision%29) (InputAction :type Input%20Action%20Object%20Reference :default "/Game/Input/IA_Look.IA_Look"))
  ;[0.15 0.15 0.15 0.5] Add Look Controls
  ;;[0.15 0.15 0.15 0.5] Left and Right
  (Pawn|Input|AddControllerYawInput (.x ActionValue))
  ;;[0.15 0.15 0.15 0.5] Up and Down
  (Pawn|Input|AddControllerPitchInput (.y ActionValue)))

(event Input|EnhancedActionEvents|EnhancedInputActionIA_Attack
  (params (ActionValue :type Boolean) (ElapsedSeconds :type Float%20%28double-precision%29) (TriggeredSeconds :type Float%20%28double-precision%29) (InputAction :type Input%20Action%20Object%20Reference :default "/Game/Input/IA_Attack.IA_Attack"))
  ;[0.15 0.15 0.15 0.5] Add Attack Input
  (:Started
    (Utilities|FlowControl|DoOnce false :!label _label
      (:Completed
        (Animation|Montage|PlayMontage (Variables|Character|GetMesh) "/Game/Gorilla/Animations/A_Gorillattackelftarm_Montage.A_Gorillattackelftarm_Montage"
          (:OnCompleted
            (goto _label Reset))
          (:OnInterrupted
            (goto _label Reset)))))))

(event EventPossessed
  (params (NewController :type Controller%20Object%20Reference))
  ;[0.15 0.15 0.15 0.5] Add Controls to Gorilla Character
  (bind _asplayer_controller (Utilities|Casting|CastToPlayerController NewController))
  (Input|AddMappingContext (PlayerController|LocalPlayerSubsystems|GetEnhancedInputLocalPlayerSubsystem _asplayer_controller) "/Game/Input/IAM_Gorilla.IAM_Gorilla" 0 "(bIgnoreAllPressedKeysUntilRelease=True,bForceImmediately=False,bNotifyUserSettings=False)"))

(event EventBeginPlay
  (bind _returnvalue (UserInterface|CreateWidget "/Game/Widgets/WB_GorillaHealth.WB_GorillaHealth_C" 0 self))
  (bind _output_get (Variables|Default|SetGorillaHUD _returnvalue))
  (UserInterface|Viewport|AddtoViewport _output_get 0))

(fn ConstructionScript)